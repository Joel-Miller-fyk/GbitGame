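; BP_Scout_Boat is a drivable boat pawn that looks like a test bed for movement and rotation.
; MoveForward smooths input with FInterpTo and heading with VInterpTo, then feeds AddMovementInput at reduced scale in reverse.
; Tick spins the actor by a fixed step every frame, independent of delta time and input.
; Keys 1 and 2 apply local or world rotation steps with debug prints; other rotation experiments are left unconnected.
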(event EventTick
  (params (DeltaSeconds :type Float%20%28single-precision%29))
  ;[1 1 1] 转向
  (Class|Actor|AddActorWorldRotation "0,10.000000, 0"))

(event Input|AxisEvents|InputAxisMoveForward
  (params (AxisValue :type Float%20%28single-precision%29))
  ;[1 1 1] 向前移动
  (Variables|Default|SetForward%20input (Math|Interpolation|FInterpTo (Variables|Default|GetForward%20input) AxisValue (Utilities|Time|GetWorldDeltaSeconds) 5.0)) ; Smooth out changes in movement input
  (Variables|Default|SetMove%20rate (Math|Interpolation|VInterpTo (Variables|Default|GetMove%20rate) (Math|Vector|GetForwardVector (Transformation|GetActorRotation)) (Utilities|Time|GetWorldDeltaSeconds) 15.0)) ; Gradually update movement direction based on actor rotation
  (Pawn|Input|AddMovementInput (Variables|Default|GetMove%20rate) (* (Math|Float|SelectFloat 0.25 1.0 (< AxisValue 0.0)) (Variables|Default|GetForward%20input)) false))

(event Input|KeyboardEvents|1
  (params (Key :type Key%20Structure :default "None"))
  (:Pressed
    (Transformation|AddActorLocalRotation "0,80.000000, 0" false false)
    (Development|PrintString "Hello")))

(event Input|KeyboardEvents|2
  (params (Key :type Key%20Structure :default "None"))
  (:Pressed
    (Class|Actor|AddActorWorldRotation "0,20.000000, 0")
    (Development|PrintString "2")))

(fn ConstructionScript)
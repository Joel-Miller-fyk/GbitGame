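; Aquarium floor grid for placing display cabins while the player boat is in Grid Mode.
; The construction script lays out grid-line meshes and an occupancy array from the plane's dimensions and cell counts.
; Tick traces under the mouse to snap the footprint, easing a preview actor there in Build mode (B toggles, 4/5/6 pick size).
; The build event spawns the cabin with a timeline scale bounce and marks cells occupied, without checking occupancy.
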(event Custom|build
  (bind _curlocation (Variables|Default|GetCurLocation))
  (bind _returnvalue (Math|Transform|MakeTransform _curlocation))
  ;[1 1 1] 建造
  (switch Utilities|FlowControl|Switch|SwitchonBuildMode (Variables|Default|GetMyBuildMode)
    (:NewEnumerator1
      (switch Utilities|FlowControl|Switch|SwitchonBuildingType (Variables|Default|GetcurBuildingType)
        (:NewEnumerator0
          (bind _returnvalue_2 (Game|SpawnActorfromClass "/Game/BP_fyk/BP_DisplayCabin.BP_DisplayCabin_C" _returnvalue "AlwaysSpawn" 0 0))
          (bind _newtrack_0 (Timeline|BuiltShake PlayFromStart)
            (:Update
              (Transformation|SetActorScale3D _returnvalue_2 (Math|Vector|Lerp(Vector) "0.800000,0.800000,0.800000" "1.200000,1.200000,1.200000" _newtrack_0)))))
        (:NewEnumerator1
          (bind _returnvalue_3 (Game|SpawnActorfromClass "/Game/BP_fyk/BP_DisplayCabin_2_1.BP_DisplayCabin_2_1_C" _returnvalue "AlwaysSpawn" 0 0))
          (bind _newtrack_0_2 (Timeline|Timeline_0 PlayFromStart)
            (:Update
              (Transformation|SetActorScale3D _returnvalue_3 (Math|Vector|Lerp(Vector) "0.800000,0.800000,0.800000" "1.200000,1.200000,1.200000" _newtrack_0_2)))))
        (:NewEnumerator2
          (bind _returnvalue_4 (Game|SpawnActorfromClass "/Game/BP_fyk/BP_DisplayCabin_2_2.BP_DisplayCabin_2_2_C" _returnvalue "AlwaysSpawn" 0 0))
          (bind _newtrack_0_3 (Timeline|Timeline_1 PlayFromStart)
            (:Update
              (Transformation|SetActorScale3D _returnvalue_4 (Math|Vector|Lerp(Vector) "0.800000,0.800000,0.800000" "1.200000,1.200000,1.200000" _newtrack_0_3))))))
      (CallFunction|SetGridSituation (Math|Vector2D|MakeVector2D (Variables|Default|GetCurBuildingXLength) (Variables|Default|GetCurBuildingYLength))))))

(event EventBeginPlay
  (bind _plane (Variables|Default|GetPlane))
  (bind _relativelocation (Variables|/Script/Engine.SceneComponent|GetRelativeLocation _plane))
  ;[1 1 1] 初始化
  (Variables|Default|SetMyBuildMode "NewEnumerator0")
  (bind _asbp_game_instance (Utilities|Casting|CastToBP_GameInstance (Game|GetGameInstance)))
  (Variables|Default|SetMyGameInstance _asbp_game_instance)
  (Variables|Default|SetCellSizeX (/ (* 2 (.x _relativelocation)) (Variables|Default|GetXCount)))
  (Variables|Default|SetCellSizeY (/ (* 2 (.y _relativelocation)) (Variables|Default|GetYCount))))

(event EventTick
  (params (DeltaSeconds :type Float%20%28single-precision%29))
  (bind _returnvalue (Transformation|GetActorLocation))
  (bind _returnvalue_2 (Game|GetPlayerController 0))
  (bind _cellsizex (Variables|Default|GetCellSizeX))
  (bind _cellsizey (Variables|Default|GetCellSizeY))
  (bind (_worldlocation _worlddirection) (Game|Player|ConvertMouseLocationToWorldSpace _returnvalue_2))
  ;[1 1 1] 获取当前指向格子位置并设置preview位置
  (switch Utilities|FlowControl|Switch|SwitchonGameMode (Variables|/Game/BP_fyk/BP_boat.BP_boat_C|GetGameMode (Variables|/Game/BP_xyl/Inventory/GameFramework/BP_GameInstance.BP_GameInstance_C|GetPlayerBoat (Variables|Default|GetMyGameInstance)))
    (:NewEnumerator3
      (bind _outhit (Collision|LineTraceByChannel _worldlocation (+ _worldlocation (* _worlddirection 10000)) "TraceTypeQuery1" false 0 "ForOneFrame" false))
      (Variables|Default|SetCurMouseCell (Math|Vector2D|MakeVector2D (Math|Conversions|ToFloat(Integer) (Math|Float|Truncate (/ (.x (- (.Location (Collision|BreakHitResult _outhit)) (Transformation|GetActorLocation))) (Variables|Default|GetCellSizeX)))) (Math|Conversions|ToFloat(Integer) (Math|Float|Truncate (/ (.y (- (.Location (Collision|BreakHitResult _outhit)) (Transformation|GetActorLocation))) (Variables|Default|GetCellSizeY))))))
      (Utilities|FlowControl|Sequence
        (:then_0
          (if (Math|Vector|Equal(Vector) (Variables|Default|GetCurLocation) (Math|Vector|MakeVector (+ (+ (* (/ (+ (.x (Variables|Default|GetCurMouseCell)) (+ (.x (Variables|Default|GetCurMouseCell)) (- (Variables|Default|GetCurBuildingXLength) 1.0))) 2.0) _cellsizex) (/ _cellsizex 2.0)) (.x _returnvalue)) (+ (+ (* (/ (+ (.y (Variables|Default|GetCurMouseCell)) (+ (.y (Variables|Default|GetCurMouseCell)) (- (Variables|Default|GetCurBuildingYLength) 1.0))) 2.0) _cellsizey) (/ _cellsizey 2.0)) (.y _returnvalue)) (.z _returnvalue)) 0.0001)
            (switch Utilities|FlowControl|Switch|SwitchonBuildMode (Variables|Default|GetMyBuildMode)
              (:NewEnumerator1
                (bind _movingline (Timeline|PreviewMoving Play)
                  (:Update
                    (Transformation|SetActorLocation (Variables|Default|GetpreviewBuilding) (Math|Vector|Lerp(Vector) (Transformation|GetActorLocation (Variables|Default|GetpreviewBuilding)) (Variables|Default|GetCurLocation) _movingline) false false)))))
            (else
              (Variables|Default|SetCurLocation (Math|Vector|MakeVector (+ (+ (* (/ (+ (.x (Variables|Default|GetCurMouseCell)) (+ (.x (Variables|Default|GetCurMouseCell)) (- (Variables|Default|GetCurBuildingXLength) 1.0))) 2.0) _cellsizex) (/ _cellsizex 2.0)) (.x _returnvalue)) (+ (+ (* (/ (+ (.y (Variables|Default|GetCurMouseCell)) (+ (.y (Variables|Default|GetCurMouseCell)) (- (Variables|Default|GetCurBuildingYLength) 1.0))) 2.0) _cellsizey) (/ _cellsizey 2.0)) (.y _returnvalue)) (.z _returnvalue)))
              (Timeline|PreviewMoving SetNewTime))))))))

(event Input|KeyboardEvents|B
  (params (Key :type Key%20Structure :default "None"))
  (bind _previewbuilding (Variables|Default|GetpreviewBuilding))
  (bind _buildingchildnum (Variables|Default|GetbuildingChildNum))
  (bind _defaultsceneroot (Variables|/Game/BP_fyk/BP_PreviewCabin.BP_PreviewCabin_C|GetDefaultSceneRoot _previewbuilding))
  (bind _returnvalue (Components|GetChildComponent _defaultsceneroot _buildingchildnum))
  ;[1 1 1] 进入建造模式
  (:Pressed
    (switch Utilities|FlowControl|Switch|SwitchonGameMode (Variables|/Game/BP_fyk/BP_boat.BP_boat_C|GetGameMode (Variables|/Game/BP_xyl/Inventory/GameFramework/BP_GameInstance.BP_GameInstance_C|GetPlayerBoat (Variables|Default|GetMyGameInstance)))
      (:NewEnumerator3
        (Utilities|FlowControl|FlipFlop
          (:A
            (Development|PrintString "buildMode")
            (Variables|Default|SetMyBuildMode "NewEnumerator1")
            (Rendering|SetVisibility _returnvalue true false))
          (:B
            (Development|PrintString "idleMode")
            (Variables|Default|SetMyBuildMode "NewEnumerator0")
            (Rendering|SetVisibility _returnvalue false false)))))))

(event Input|KeyboardEvents|4
  (params (Key :type Key%20Structure :default "None"))
  ;[1 1 1] 改变建筑类型
  (:Pressed
    (CallFunction|ChangeBuildingType "NewEnumerator0")))

(event Input|KeyboardEvents|5
  (params (Key :type Key%20Structure :default "None"))
  ;[1 1 1] 改变建筑类型
  (:Pressed
    (CallFunction|ChangeBuildingType "NewEnumerator1")))

(event Input|KeyboardEvents|6
  (params (Key :type Key%20Structure :default "None"))
  ;[1 1 1] 改变建筑类型
  (:Pressed
    (CallFunction|ChangeBuildingType "NewEnumerator2")))

(fn ConstructionScript
  (bind _xcount (Variables|Default|GetXCount))
  (bind _ycount (Variables|Default|GetYCount))
  (bind _plane (Variables|Default|GetPlane))
  (bind _relativelocation (Variables|/Script/Engine.SceneComponent|GetRelativeLocation _plane))
  (bind _relativescale3d (Variables|/Script/Engine.SceneComponent|GetRelativeScale3D _plane))
  (Utilities|FlowControl|Sequence
    (:then_0
      (for _index (range 0 (Math|Float|Truncate _xcount))
        (bind _returnvalue (AddComponent|AddStaticMeshComponent false (Math|Transform|MakeTransform (Math|Vector|MakeVector (* _index (/ (* 2 (.x _relativelocation)) _xcount)) (.y _relativelocation) (+ (.z _relativelocation) 1.0)) "0, 0, 0" (Math|Vector|MakeVector 0.2 (.y _relativescale3d) 1.0))))
        (Utilities|Array|SetArrayElem (Variables|Default|GetLines) _index _returnvalue)))
    (:then_1
      (for _index_2 (range 0 (Math|Float|Truncate _ycount))
        (AddComponent|AddStaticMeshComponent false (Math|Transform|MakeTransform (Math|Vector|MakeVector (.x _relativelocation) (* _index_2 (/ (* 2 (.y _relativelocation)) _ycount)) (+ (.z _relativelocation) 1.0)) "0, 0, 0" (Math|Vector|MakeVector (.x _relativescale3d) 0.2 1.0)))))
    (:then_2
      (Variables|Default|SetcurBuildingType "NewEnumerator0")
      (Variables|Default|SetCurBuildingXLength 1.0)
      (Variables|Default|SetCurBuildingYLength 1.0)
      (for _index_3 (range 0 (Math|Float|Truncate (Variables|Default|GetXCount)))
        (for _index_4 (range 0 (Math|Float|Truncate (Variables|Default|GetYCount)))
          (Utilities|Array|Add (Variables|Default|GetGridSituation) false))))))

(fn ChangeBuildingType
  (params (NewParam :type BuildingType%20Enum :default "NewEnumerator0"))
  (bind _previewbuilding (Variables|Default|GetpreviewBuilding))
  (bind _defaultsceneroot (Variables|/Game/BP_fyk/BP_PreviewCabin.BP_PreviewCabin_C|GetDefaultSceneRoot _previewbuilding))
  (switch Utilities|FlowControl|Switch|SwitchonBuildMode (Variables|Default|GetMyBuildMode)
    (:NewEnumerator1
      (switch Utilities|FlowControl|Switch|SwitchonBuildingType NewParam
        (:NewEnumerator0
          (Variables|Default|SetbuildingChildNum 2)
          (Variables|Default|SetCurBuildingXLength 1.0)
          (Variables|Default|SetCurBuildingYLength 1.0))
        (:NewEnumerator1
          (Variables|Default|SetbuildingChildNum 1)
          (Variables|Default|SetCurBuildingXLength 2.0)
          (Variables|Default|SetCurBuildingYLength 1.0))
        (:NewEnumerator2
          (Variables|Default|SetbuildingChildNum 0)
          (Variables|Default|SetCurBuildingXLength 2.0)
          (Variables|Default|SetCurBuildingYLength 2.0)))
      (Variables|Default|SetcurBuildingType NewParam)
      (for _index (range 0 (- (Class|SceneComponent|GetNumChildrenComponents _defaultsceneroot) 1))
        (Rendering|SetVisibility (Components|GetChildComponent _defaultsceneroot _index) false false)
        (Rendering|SetVisibility (Components|GetChildComponent _defaultsceneroot (Variables|Default|GetbuildingChildNum)) true false)))))

(fn SetGridSituation
  (params (NewParam :type Vector%202D%20Structure))
  (bind _curmousecell (Variables|Default|GetCurMouseCell))
  (for _index (range (Math|Float|Truncate (.x _curmousecell)) (Math|Float|Truncate (+ (.x _curmousecell) (- (.x NewParam) 1.0))))
    (for _index_2 (range (Math|Float|Truncate (.y _curmousecell)) (Math|Float|Truncate (+ (.y _curmousecell) (- (.y NewParam) 1.0))))
      (Utilities|Array|SetArrayElem (Variables|Default|GetGridSituation) (+ _index (Math|Float|Truncate (* _index_2 (Variables|Default|GetXCount)))) true))))
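; Player boat for a fishing game, switching between sailing, side-view fishing and aquarium grid building, while also running the day/night clock and sun height.
; Fishing projects the cursor trace onto the boat's vertical plane to aim spline-mesh lines, whose spread widens with mouse movement.
; Clicking fires a timeline-driven hook at a random angle within that spread.
; A catch starts a tug-bar minigame: F counters fish drag, and leaving the tolerance band releases it.
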(event Custom|hookBackEvent
  (bind _curcatchedfish (Variables|Default|GetcurCatchedFish))
  (bind _mygameinstance (Variables|Default|GetMyGameInstance))
  (bind _dragtolerancevalue (Utilities|Struct|Breakstruct_fishType _curcatchedfish))
  (bind _playerui (Variables|/Game/BP_xyl/Inventory/GameFramework/BP_GameInstance.BP_GameInstance_C|GetPlayerUI _mygameinstance))
  (bind _returnvalue (/ _dragtolerancevalue 2.0))
  (bind _bp_fishcaughtplay (Variables|/Game/BP_fyk/BP_UI/BP_PlayerUI.BP_PlayerUI_C|GetBP_fishCaughtPlay _playerui))
  (bind _playerbar (Variables|/Game/BP_fyk/BP_UI/BP_fishCaughtPlay.BP_fishCaughtPlay_C|GetplayerBar _bp_fishcaughtplay))
  (bind _returnvalue_2 (Class|WidgetLayoutLibrary|SlotasCanvasSlot _playerbar))
  (bind _returnvalue_3 (Class|CanvasPanelSlot|GetPosition _returnvalue_2))
  (bind _returnvalue_4 (Class|CanvasPanelSlot|GetSize _returnvalue_2))
  (bind _returnvalue_5 (* (.x _returnvalue_4) _returnvalue))
  (Development|PrintString "hookBack")
  (Variables|Default|SetisStartPlay true)
  (Progress|SetPercent _playerbar 0.5)
  (Class|CanvasPanelSlot|SetPosition (Class|WidgetLayoutLibrary|SlotasCanvasSlot (Variables|/Game/BP_fyk/BP_UI/BP_fishCaughtPlay.BP_fishCaughtPlay_C|GetL_boundary _bp_fishcaughtplay)) (Math|Vector2D|MakeVector2D (- (.x _returnvalue_3) _returnvalue_5) (.y _returnvalue_3)))
  (Class|CanvasPanelSlot|SetPosition (Class|WidgetLayoutLibrary|SlotasCanvasSlot (Variables|/Game/BP_fyk/BP_UI/BP_fishCaughtPlay.BP_fishCaughtPlay_C|GetR_boundary _bp_fishcaughtplay)) (Math|Vector2D|MakeVector2D (+ (.x _returnvalue_3) _returnvalue_5) (.y _returnvalue_3)))
  (Default|ShowUI _bp_fishcaughtplay))

(event Custom|AddOneDay
  ;[1 1 1] 计时器
  (Variables|Default|SetDayTimer (- (Variables|Default|GetTimePerDay) 1.0)))

(event Custom|hookFinishBackEvent
  (Variables|Default|SetisStartPlay false)
  (Default|HideUI (Variables|/Game/BP_fyk/BP_UI/BP_PlayerUI.BP_PlayerUI_C|GetBP_fishCaughtPlay (Variables|/Game/BP_xyl/Inventory/GameFramework/BP_GameInstance.BP_GameInstance_C|GetPlayerUI (Variables|Default|GetMyGameInstance)))))

(event Custom|AddOneHour
  ;[1 1 1] 计时器
  (Variables|Default|SetDayTimer (+ (Variables|Default|GetDayTimer) (/ (Variables|Default|GetTimePerDay) 24.0))))

(event EventBeginPlay
  ;[1 1 1] 初始化
  (Variables|Default|SetGameMode "NewEnumerator0")
  (bind _asbp_game_instance (Utilities|Casting|CastToBP_GameInstance (Game|GetGameInstance)))
  (Variables|Default|SetMyGameInstance _asbp_game_instance))

(event EventTick
  (params (DeltaSeconds :type Float%20%28single-precision%29))
  (bind _returnvalue (Game|GetPlayerController 0))
  (bind _returnvalue_2 (Game|GetPlayerController 0))
  (bind _returnvalue_3 (Transformation|GetActorRotation))
  (bind _testspline (Variables|Default|GettestSpline))
  (bind _mygameinstance (Variables|Default|GetMyGameInstance))
  (bind _curcatchedfish (Variables|Default|GetcurCatchedFish))
  (bind _aimlinelength (Variables|Default|GetAimLineLength))
  (bind _maxoffset_angle (Variables|Default|GetMaxOffset%20Angle))
  (bind _mygameinstance_2 (Variables|Default|GetMyGameInstance))
  (bind _skysphere (Variables|Default|GetSkySphere))
  (bind (_fishname _speedmin _speedmax _saleprice _viewvalue _generaterate _description _generatedepthmin _generatedepthmax _dragtolerancevalue _dragforce) (Utilities|Struct|Breakstruct_fishType _curcatchedfish))
  (bind (_locationx _locationy) (Game|Player|GetMousePosition _returnvalue))
  (bind (_location _tangent) (Spline|GetLocationandTangentatSplinePoint _testspline 0 "Local"))
  (bind (_location_2 _tangent_2) (Spline|GetLocationandTangentatSplinePoint _testspline 1 "Local"))
  (bind (_worldlocation _worlddirection) (Game|Player|ConvertMouseLocationToWorldSpace _returnvalue_2))
  (bind _returnvalue_4 (Math|Vector|GetForwardVector _returnvalue_3))
  (bind _returnvalue_5 (- _aimlinelength 4e+02))
  (bind _playerui (Variables|/Game/BP_xyl/Inventory/GameFramework/BP_GameInstance.BP_GameInstance_C|GetPlayerUI _mygameinstance))
  (bind _playerui_2 (Variables|/Game/BP_xyl/Inventory/GameFramework/BP_GameInstance.BP_GameInstance_C|GetPlayerUI _mygameinstance_2))
  (bind _returnvalue_6 (Math|Vector2D|MakeVector2D _locationx _locationy))
  (bind _returnvalue_7 (- _location_2 _location))
  (bind _bp_fishcaughtplay (Variables|/Game/BP_fyk/BP_UI/BP_PlayerUI.BP_PlayerUI_C|GetBP_fishCaughtPlay _playerui_2))
  (bind _returnvalue_8 (Math|Vector|Normalize _returnvalue_7))
  (bind _playerbar (Variables|/Game/BP_fyk/BP_UI/BP_fishCaughtPlay.BP_fishCaughtPlay_C|GetplayerBar _bp_fishcaughtplay))
  (bind _returnvalue_9 (* _returnvalue_8 _returnvalue_5))
  (bind _percent (Variables|/Script/UMG.ProgressBar|GetPercent _playerbar))
  (bind _returnvalue_10 (- _percent _dragforce))
  (bind _returnvalue_11 (+ _location _returnvalue_9))
  ;[1 1 1] 瞄准线/tick
  (Utilities|FlowControl|Sequence
    (:then_0
      (switch Utilities|FlowControl|Switch|SwitchonGameMode (Variables|Default|GetGameMode)
        (:NewEnumerator1
          (bind _outhit (Collision|LineTraceByChannel _worldlocation (+ _worldlocation (* _worlddirection 10000)) "TraceTypeQuery1" false 0 "None"))
          (bind _output_get (Variables|Default|SetAimAngle (Class|KismetMathLibrary|DegAcos (/ (Math|Vector|DotProduct (Class|KismetMathLibrary|ProjectPointontoPlane (- (.Location (Collision|BreakHitResult _outhit)) (Transformation|GetActorLocation)) _returnvalue_4 (Math|Vector|GetRightVector _returnvalue_3)) (- "0, 0, 0" _returnvalue_4)) (Math|Vector|VectorLength (Class|KismetMathLibrary|ProjectPointontoPlane (- (.Location (Collision|BreakHitResult _outhit)) (Transformation|GetActorLocation)) _returnvalue_4 (Math|Vector|GetRightVector _returnvalue_3)))))))
          (Utilities|FlowControl|Sequence
            (:then_0
              (Spline|SetLocationatSplinePoint (Variables|Default|GettestSpline) 1 (Math|Vector|RotateVectorAroundAxis (Math|Vector|MakeVector -1.0 0.0 0.0) _output_get "0.000000,-1.000000,0.000000") "Local" true)
              (SplineMesh|SetStartandEnd (Variables|Default|GetLineMesh) _location _tangent (+ _location (* _returnvalue_8 _aimlinelength)) _tangent_2 true :!class /Script/Engine.SplineMeshComponent)
              (SplineMesh|SetStartandEnd (Variables|Default|GetLineMesh_left) _location _tangent (Math|Vector|RotateVectorAroundAxis _returnvalue_11 (Variables|Default|GetOffset%20Angle) "0.000000,-1.000000,0.000000") _tangent_2 true :!class /Script/Engine.SplineMeshComponent)
              (SplineMesh|SetStartandEnd (Variables|Default|GetLineMesh_right) _location _tangent (Math|Vector|RotateVectorAroundAxis _returnvalue_11 (- 0.0 (Variables|Default|GetOffset%20Angle)) "0.000000,-1.000000,0.000000") _tangent_2 true :!class /Script/Engine.SplineMeshComponent))))))
    (:then_1
      ;[1 1 1] 瞄准散度
      (if (> (* (Math|Vector2D|Vector2DLength (- _returnvalue_6 (Variables|Default|GetpreviousMousePosition))) 0.05) 0.1)
        (if (< (Variables|Default|GetOffset%20Angle) _maxoffset_angle)
          (Variables|Default|SetOffset%20Angle (+ (Variables|Default|GetOffset%20Angle) (Math|Float|%(Float) (* (Math|Vector2D|Vector2DLength (- _returnvalue_6 (Variables|Default|GetpreviousMousePosition))) 0.05) _maxoffset_angle))))
        (Variables|Default|SetstartShrink false)
        (Variables|Default|SetpreviousMousePosition _returnvalue_6 :!label _label)
        (elif (> (Variables|Default|GetOffset%20Angle) 0.0)
          (if (Variables|Default|GetstartShrink)
            (Variables|Default|SetOffset%20Angle (- (Variables|Default|GetOffset%20Angle) 1.0))
            (goto _label)
            (else
              (Utilities|FlowControl|Delay 0.1)
              (Variables|Default|SetstartShrink true))))))
    (:then_2
      (if (Variables|Default|GetisStartPlay)
        (Utilities|FlowControl|Sequence
          (:then_0
            (Progress|SetPercent _playerbar _returnvalue_10)
            (bind _output_get_2 (Variables|Default|SetcurPlayPercent _returnvalue_10)))
          (:then_1
            (if (or (< _output_get_2 (/ (- 1.0 _dragtolerancevalue) 2.0)) (> _output_get_2 (/ (+ 1.0 _dragtolerancevalue) 2.0)))
              (Utilities|FlowControl|DoOnce false :!label _label_2
                (:Completed
                  (Development|PrintString "drayfail")
                  (Default|DisAttachFish (Variables|Default|GetcurCatchedFish_BP))
                  (CallFunction|HookFinishBackEvent)))
              (else
                (goto _label_2 Reset)))))))
    (:then_3
      ;[1 1 1] 计时器
      (if (> (Variables|Default|GetDayTimer) (Variables|Default|GetTimePerDay))
        (bind _output_get_3 (Variables|Default|SetDay (+ (Variables|Default|GetDay) 1.0)))
        (Development|PrintString (Utilities|String|ToString(Float) _output_get_3))
        (Default|SetDay _playerui (Utilities|Text|ToText(Float) _output_get_3 "HalfToEven"))
        (Variables|Default|SetDayTimer 0.0)
        (else
          (bind _output_get_4 (Variables|Default|SetDayTimer (+ (Variables|Default|GetDayTimer) (* (Utilities|Time|GetWorldDeltaSeconds) (Variables|Default|GetTestTimeFaster)))))
          (bind _output_get_5 (Variables|Default|SetShowDayTime (Math|Conversions|ToFloat(Integer) (Math|Float|Truncate (/ _output_get_4 (/ (Variables|Default|GetTimePerDay) 24.0))))))
          (Default|SetTime _playerui (Utilities|Text|ToText(Float) _output_get_5 "HalfToEven"))
          (Variables|/Engine/EngineSky/BP_Sky_Sphere.BP_Sky_Sphere_C|SetSun%20height _skysphere (Math|Curves|GetFloatValue (Variables|Default|GetTimeCurve) (/ (Variables|Default|GetDayTimer) (/ (Variables|Default|GetTimePerDay) 4.0))))
          (Default|RefreshMaterial _skysphere))))))

(event Input|AxisEvents|InputAxisMoveForward
  (params (AxisValue :type Float%20%28single-precision%29))
  ;[1 1 1] Movement and Rotation
  (switch Utilities|FlowControl|Switch|SwitchonGameMode (Variables|Default|GetGameMode)
    (:NewEnumerator0
      (bind _output_get (Variables|Default|SetForward%20Input (Math|Interpolation|FInterpTo (Variables|Default|GetForward%20Input) AxisValue (Utilities|Time|GetWorldDeltaSeconds) 2.0)))
      (Transformation|AddActorWorldOffset (* (Math|Vector|GetForwardVector (Transformation|GetActorRotation)) (* _output_get (Variables|Default|GetMove%20Speed)))))))

(event Input|AxisEvents|InputAxisMoveRight
  (params (AxisValue :type Float%20%28single-precision%29))
  ;[1 1 1] Movement and Rotation
  (switch Utilities|FlowControl|Switch|SwitchonGameMode (Variables|Default|GetGameMode)
    (:NewEnumerator0
      (bind _output_get (Variables|Default|SetRight%20Input (Math|Interpolation|FInterpTo (Variables|Default|GetRight%20Input) AxisValue (Utilities|Time|GetWorldDeltaSeconds) 2.0)))
      (Transformation|AddActorLocalRotation (Math|Rotator|MakeRotator 0.0 0.0 (* (Variables|Default|GetRotate%20Spped) _output_get)) false false))))

(event Input|KeyboardEvents|2
  (params (Key :type Key%20Structure :default "None"))
  (bind _camera (Variables|Default|GetCamera))
  (bind _camera_2 (Variables|Default|GetCamera))
  (bind _springarm (Variables|Default|GetSpringArm))
  (bind _springarm_2 (Variables|Default|GetSpringArm))
  ;[1 1 1] 视角转换
  (:Pressed
    (switch Utilities|FlowControl|Switch|SwitchonGameMode (Variables|Default|GetGameMode)
      (:NewEnumerator0
        (bind _newtrack_0 (Timeline|blenderCamera PlayFromStart)
          (:Update
            (Transformation|SetRelativeLocation _springarm_2 (Math|Vector|Lerp(Vector) (Variables|/Script/Engine.SceneComponent|GetRelativeLocation _springarm_2) "-1080.000000,0.000000,-640.000000" _newtrack_0) false false)
            (Transformation|SetRelativeRotation _springarm_2 (Math|Rotator|Lerp(Rotator) (Variables|/Script/Engine.SceneComponent|GetRelativeRotation _springarm_2) "0,-90.000000, 0" _newtrack_0) false false)
            (Variables|/Script/Engine.SpringArmComponent|SetTargetArmLength _springarm_2 (Math|Float|Lerp (Variables|/Script/Engine.SpringArmComponent|GetTargetArmLength _springarm_2) 6.4e+03 _newtrack_0))
            (Camera|SetFieldOfView _camera_2 (Math|Float|Lerp (Variables|/Script/Engine.CameraComponent|GetFieldOfView _camera_2) 3e+01 _newtrack_0)))
          (:Finished
            (Variables|/Script/Engine.PlayerController|SetbShowMouseCursor (Game|GetPlayerController 0) true)
            (Variables|Default|SetGameMode "NewEnumerator1")
            (Rendering|SetVisibility (Variables|Default|GetLineMesh) true false)
            (Variables|Default|SetOffset%20Angle 3e+01)
            (Development|PrintString (Utilities|String|EnumtoString (Variables|Default|GetGameMode)))
            (Variables|Default|SetTestTimeFaster 2.0))))
      (:NewEnumerator1
        (Utilities|FlowControl|Sequence
          (:then_0
            (bind _newtrack_0_2 (Timeline|Timeline_0 PlayFromStart)
              (:Update
                (Transformation|SetRelativeLocation _springarm (Math|Vector|Lerp(Vector) (Variables|/Script/Engine.SceneComponent|GetRelativeLocation _springarm) "0.000000, 0,420.000000" _newtrack_0_2) false false)
                (Transformation|SetRelativeRotation _springarm (Math|Rotator|Lerp(Rotator) (Variables|/Script/Engine.SceneComponent|GetRelativeRotation _springarm) "-10.000000,0.000000, 0" _newtrack_0_2) false false)
                (Variables|/Script/Engine.SpringArmComponent|SetTargetArmLength _springarm (Math|Float|Lerp (Variables|/Script/Engine.SpringArmComponent|GetTargetArmLength _springarm) 1.4e+03 _newtrack_0_2))
                (Camera|SetFieldOfView _camera (Math|Float|Lerp (Variables|/Script/Engine.CameraComponent|GetFieldOfView _camera) 9e+01 _newtrack_0_2)))
              (:Finished
                (Variables|Default|SetGameMode "NewEnumerator0")
                (Development|PrintString (Utilities|String|EnumtoString (Variables|Default|GetGameMode)))
                (Variables|Default|SetTestTimeFaster 1.0))))
          (:then_1
            (Variables|/Script/Engine.PlayerController|SetbShowMouseCursor (Game|GetPlayerController 0) false)
            (Rendering|SetVisibility (Variables|Default|GetLineMesh) false false)))))))

(event Input|KeyboardEvents|1
  (params (Key :type Key%20Structure :default "None"))
  ;[1 1 1] 生成鱼测试
  (:Pressed
    (Default|GenerateFish (Variables|/Game/BP_xyl/Inventory/GameFramework/BP_GameInstance.BP_GameInstance_C|GetGeneratePanel (Variables|Default|GetMyGameInstance)))))

(event Input|KeyboardEvents|F
  (params (Key :type Key%20Structure :default "None"))
  (bind _mygameinstance (Variables|Default|GetMyGameInstance))
  (bind _playerui (Variables|/Game/BP_xyl/Inventory/GameFramework/BP_GameInstance.BP_GameInstance_C|GetPlayerUI _mygameinstance))
  (bind _bp_fishcaughtplay (Variables|/Game/BP_fyk/BP_UI/BP_PlayerUI.BP_PlayerUI_C|GetBP_fishCaughtPlay _playerui))
  (bind _playerbar (Variables|/Game/BP_fyk/BP_UI/BP_fishCaughtPlay.BP_fishCaughtPlay_C|GetplayerBar _bp_fishcaughtplay))
  ;[1 1 1] 小游戏
  (:Pressed
    (Utilities|FlowControl|Sequence
      (:then_0
        (Progress|SetPercent _playerbar (+ (Variables|/Script/UMG.ProgressBar|GetPercent _playerbar) (Variables|Default|GetcurPullNum)))))))

(event Input|KeyboardEvents|G
  (params (Key :type Key%20Structure :default "None"))
  ;[1 1 1] 生成鱼测试
  (:Pressed
    (Default|GenerateNumFish (Variables|/Game/BP_xyl/Inventory/GameFramework/BP_GameInstance.BP_GameInstance_C|GetGeneratePanel (Variables|Default|GetMyGameInstance)) 10)))

(event Input|KeyboardEvents|3
  (params (Key :type Key%20Structure :default "None"))
  (bind _returnvalue (Game|GetPlayerController 0))
  ;[1 1 1] 视角切换2
  (:Pressed
    (switch Utilities|FlowControl|Switch|SwitchonGameMode (Variables|Default|GetGameMode)
      (:NewEnumerator0
        (Variables|Default|SetGameMode "NewEnumerator3")
        (Game|Player|SetViewTargetwithBlend _returnvalue (Variables|Default|GetAquariumCamera_ver2) 1.0 "VTBlend_Linear" 0.0 false)
        (Variables|/Script/Engine.PlayerController|SetbShowMouseCursor (Game|GetPlayerController 0) true))
      (:NewEnumerator3
        (Variables|/Script/Engine.PlayerController|SetbShowMouseCursor (Game|GetPlayerController 0) false)
        (Game|Player|SetViewTargetwithBlend _returnvalue self 1.0 "VTBlend_Linear" 0.0 false)
        (Variables|Default|SetGameMode "NewEnumerator0")))))

(event Input|MouseEvents|LeftMouseButton
  (params (Key :type Key%20Structure :default "None"))
  (bind _testspline (Variables|Default|GettestSpline))
  (bind _offset_angle (Variables|Default|GetOffset%20Angle))
  (bind _testspline_2 (Variables|Default|GettestSpline))
  (bind (_location _tangent) (Spline|GetLocationandTangentatSplinePoint _testspline 0 "Local"))
  ;[1 1 1] 发射鱼钩
  (:Pressed
    (if (Variables|Default|GetisHookBack)
      (switch Utilities|FlowControl|Switch|SwitchonGameMode (Variables|Default|GetGameMode)
        (:NewEnumerator1
          (Variables|Default|SetLunchAngle (Math|Random|RandomFloatinRange (- 0.0 _offset_angle) _offset_angle))
          (Variables|Default|SetLunchDirection (Math|Vector|RotateVectorAroundAxis (Math|Vector|Normalize (- (.Location (Spline|GetLocationandTangentatSplinePoint _testspline_2 1 "Local")) (.Location (Spline|GetLocationandTangentatSplinePoint _testspline_2 0 "Local")))) (Variables|Default|GetLunchAngle) "0.000000,-1.000000,0.000000"))
          (Utilities|FlowControl|Sequence
            (:then_0
              (bind _newtrack_0 (Timeline|HookLunch PlayFromStart)
                (:Update
                  (Utilities|FlowControl|Sequence :!label _label
                    (:then_0
                      (if (Variables|Default|GetisFishCaught)
                        (Variables|Default|SetcurHookVar (stale _newtrack_0_2))
                        (else
                          (Variables|Default|SetcurHookVar _newtrack_0)))
                      (SplineMesh|SetStartandEnd (Variables|Default|GetHook) _location _tangent (Math|Vector|RotateVectorAroundAxis (+ _location (* (Variables|Default|GetLunchDirection) (Math|Float|Lerp 0.0 (Variables|Default|GetHookLength) (Variables|Default|GetcurHookVar)))) (Variables|Default|GetLunchAngle) "0.000000,-1.000000,0.000000") (.Tangent (Spline|GetLocationandTangentatSplinePoint _testspline 1 "Local")) true :!class /Script/Engine.SplineMeshComponent)
                      (Transformation|SetRelativeLocation (Variables|Default|GetfishHook) (Math|Vector|RotateVectorAroundAxis (+ _location (* (Variables|Default|GetLunchDirection) (Math|Float|Lerp 0.0 (Variables|Default|GetHookLength) (Variables|Default|GetcurHookVar)))) (Variables|Default|GetLunchAngle) "0.000000,-1.000000,0.000000") false false)
                      (Variables|Default|SetFishHookLocation (Math|Vector|RotateVectorAroundAxis (+ _location (* (Variables|Default|GetLunchDirection) (Math|Float|Lerp 0.0 (Variables|Default|GetHookLength) (Variables|Default|GetcurHookVar)))) (Variables|Default|GetLunchAngle) "0.000000,-1.000000,0.000000")))
                    (:then_1
                      (if (Variables|Default|GetisFishCaught)
                        (if (> (Variables|Default|GetcurHookVar) 0.0) :!label _label_2
                          (Utilities|FlowControl|DoOnce false :!label _label_3
                            (:Completed
                              (if (Variables|Default|GetisFishCaught)
                                (Utilities|FlowControl|Sequence
                                  (:then_0
                                    (Timeline|HookLunch Stop))
                                  (:then_1
                                    (bind _newtrack_0_2 (Timeline|HookBack SetNewTime)
                                      (:Update
                                        (goto _label))
                                      (:Finished
                                        (goto _label_2))))
                                  (:then_2
                                    (Variables|Default|SethookLunchorBack false)
                                    (Timeline|HookBack Play))
                                  (:then_3
                                    (CallFunction|HookBackEvent)))
                                (else
                                  (Variables|Default|SethookLunchorBack false)
                                  (Timeline|HookLunch Reverse)))))
                          (else
                            (Variables|Default|SetisHookBack true)
                            (Variables|Default|SetisFishCaught false)
                            (CallFunction|HookFinishBackEvent)))))))
                (:Finished
                  (goto _label_2))))
            (:then_1
              (Variables|Default|SetisHookBack false)
              (Variables|Default|SethookLunchorBack true)
              (goto _label_3 Reset))))
        (:NewEnumerator3
          (Default|BuildVer2 (Variables|Default|GetAcquariumFloor_ver2)))))))

(event Input|KeyboardEvents|J
  (params (Key :type Key%20Structure :default "None"))
  ;[1 1 1] 计时器
  (:Pressed
    (CallFunction|AddOneHour)))

(fn ConstructionScript
  (Utilities|FlowControl|Sequence
    (:then_1
      (bind _returnvalue (AddComponent|AddSplineMeshComponent false))
      (bind _output_get (Variables|Default|SetLineMesh _returnvalue))
      (SplineMesh|SetStartScale _output_get "(X=0.100000,Y=0.100000)" true :!class /Script/Engine.SplineMeshComponent)
      (SplineMesh|SetEndScale _output_get "(X=0.100000,Y=0.100000)" true :!class /Script/Engine.SplineMeshComponent))
    (:then_2
      (bind _returnvalue_2 (AddComponent|AddSplineMeshComponent false))
      (bind _output_get_2 (Variables|Default|SetLineMesh_left _returnvalue_2))
      (SplineMesh|SetStartScale _output_get_2 "(X=0.100000,Y=0.100000)" true :!class /Script/Engine.SplineMeshComponent)
      (SplineMesh|SetEndScale _output_get_2 "(X=0.100000,Y=0.100000)" true :!class /Script/Engine.SplineMeshComponent))
    (:then_3
      (bind _returnvalue_3 (AddComponent|AddSplineMeshComponent false))
      (bind _output_get_3 (Variables|Default|SetLineMesh_right _returnvalue_3))
      (SplineMesh|SetStartScale _output_get_3 "(X=0.100000,Y=0.100000)" true :!class /Script/Engine.SplineMeshComponent)
      (SplineMesh|SetEndScale _output_get_3 "(X=0.100000,Y=0.100000)" true :!class /Script/Engine.SplineMeshComponent))
    (:then_4
      (bind _returnvalue_4 (AddComponent|AddSplineMeshComponent false))
      (bind _output_get_4 (Variables|Default|SetHook _returnvalue_4))
      (SplineMesh|SetStartScale _output_get_4 "(X=0.150000,Y=0.150000)" true :!class /Script/Engine.SplineMeshComponent)
      (SplineMesh|SetEndScale _output_get_4 "(X=0.150000,Y=0.150000)" true :!class /Script/Engine.SplineMeshComponent))))

(fn Reconstruction
  (bind _number_of_meshes (Variables|Default|GetNumber%20of%20meshes))
  (if (> _number_of_meshes 0)
    (bind _output_get (Variables|Default|SetLastIndex (- _number_of_meshes 1)))
    (for _index (range 0 _output_get) ; Repeat loop for each mesh to add
      (Components|InstancedStaticMesh|UpdateInstanceTransform (Variables|Default|GetLine) _index (|Transform_2_2 (* _index (/ (Spline|GetSplineLength (Variables|Default|GetSpline)) (Math|Conversions|ToFloat(Integer) (Variables|Default|GetLastIndex)))) 0.4) false (== _index (Variables|Default|GetLastIndex)) false))))
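; Aquarium floor grid where the player places and removes buildings, stocks them with fish and totals their income.
; Construction script draws grid lines and sizes a flat boolean occupancy array.
; In the boat's Grid Mode, Tick traces the mouse to a cell and eases previews toward it via timelines.
; Build, Destroy and PutFish modes drive Build_ver2, using data-table types to spawn BP_Building, free cells or add fish.
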(event Custom|EnterPutMode
  (bind _mybuildmode (Variables|Default|GetMyBuildMode))
  ;[1 1 1] 进入放鱼模式
  (switch Utilities|FlowControl|Switch|SwitchonGameMode (Variables|/Game/BP_fyk/BP_boat.BP_boat_C|GetGameMode (Variables|/Game/BP_xyl/Inventory/GameFramework/BP_GameInstance.BP_GameInstance_C|GetPlayerBoat (Variables|Default|GetMyGameInstance)))
    (:NewEnumerator3
      (if (Utilities|Enum|Equal(Enum) _mybuildmode "NewEnumerator3")
        (CallFunction|ExitCurBuildMode _mybuildmode)
        (CallFunction|ChangeMode "NewEnumerator0")
        (Development|PrintString "Idle")
        (else
          (CallFunction|ExitCurBuildMode _mybuildmode)
          (CallFunction|ChangeMode "NewEnumerator3")
          (Development|PrintString "PutFish"))))))

(event Custom|Build_ver2
  (bind _returnvalue (Game|GetPlayerController 0))
  (bind _returnvalue_2 (Game|GetPlayerController 0))
  (bind _curfishinfo (Variables|Default|GetCurFishInfo))
  (bind _buildings (Variables|Default|GetBuildings))
  (bind _buildings_2 (Variables|Default|GetBuildings))
  (bind _curmousecell (Variables|Default|GetCurMouseCell))
  (bind _curbuildinginfo (Variables|Default|GetCurBuildingInfo))
  (bind (_worldlocation _worlddirection) (Game|Player|ConvertMouseLocationToWorldSpace _returnvalue))
  (bind (_worldlocation_2 _worlddirection_2) (Game|Player|ConvertMouseLocationToWorldSpace _returnvalue_2))
  ;[1 1 1] 建造
  (switch Utilities|FlowControl|Switch|SwitchonBuildMode (Variables|Default|GetMyBuildMode)
    (:NewEnumerator1
      (bind _canbuild (CallFunction|CheckGrid))
      (if _canbuild
        (bind _returnvalue_3 (Game|SpawnActorfromClass "/Game/BP_fyk/BP_Building.BP_Building_C" (Math|Transform|MakeTransform (Variables|Default|GetCurLocation)) "AlwaysSpawn" 0 0))
        (Components|StaticMesh|SetStaticMesh (Variables|/Game/BP_fyk/BP_Building.BP_Building_C|GetBuilding _returnvalue_3) (.mesh _curbuildinginfo))
        (Variables|/Game/BP_fyk/BP_Building.BP_Building_C|SetXposition _returnvalue_3 (.x _curmousecell))
        (Variables|/Game/BP_fyk/BP_Building.BP_Building_C|SetYposition _returnvalue_3 (.y _curmousecell))
        (Variables|/Game/BP_fyk/BP_Building.BP_Building_C|SetXLength _returnvalue_3 (.xlength _curbuildinginfo))
        (Variables|/Game/BP_fyk/BP_Building.BP_Building_C|SetYLength _returnvalue_3 (.ylength _curbuildinginfo))
        (Variables|/Game/BP_fyk/BP_Building.BP_Building_C|SetFishCapacity _returnvalue_3 (.fishcapacity _curbuildinginfo))
        (Variables|/Game/BP_fyk/BP_Building.BP_Building_C|SetViewValueTimes _returnvalue_3 (.viewvaluetimes _curbuildinginfo))
        (Variables|/Game/BP_fyk/BP_Building.BP_Building_C|SetMaintainCost _returnvalue_3 (.maintaincost _curbuildinginfo))
        (CallFunction|SetGridSituation (Math|Vector2D|MakeVector2D (Variables|Default|GetCurBuildingXLength) (Variables|Default|GetCurBuildingYLength)))
        (Utilities|Array|Add _buildings_2 _returnvalue_3)
        (Development|PrintString (Utilities|String|ToString(Integer) (Utilities|Array|Length _buildings_2)))
        (Transformation|SetWorldScale3D (Variables|/Game/BP_fyk/BP_Building.BP_Building_C|GetBuilding _returnvalue_3) (Math|Vector|MakeVector (* (.x (Transformation|GetWorldScale (Variables|/Game/BP_fyk/BP_Building.BP_Building_C|GetBuilding _returnvalue_3))) (Variables|/Game/BP_fyk/BP_Building.BP_Building_C|GetXLength _returnvalue_3)) (* (.y (Transformation|GetWorldScale (Variables|/Game/BP_fyk/BP_Building.BP_Building_C|GetBuilding _returnvalue_3))) (Variables|/Game/BP_fyk/BP_Building.BP_Building_C|GetYLength _returnvalue_3)) (.z (Transformation|GetWorldScale (Variables|/Game/BP_fyk/BP_Building.BP_Building_C|GetBuilding _returnvalue_3)))))
        (else
          (Development|PrintString "You can't build here!")
          (CallFunction|PrintOcupidGridNum))))
    (:NewEnumerator2
      ;[1 1 1] 销毁
      (bind _outhit (Collision|LineTraceByChannel _worldlocation_2 (+ _worldlocation_2 (* _worlddirection_2 10000)) "TraceTypeQuery1" false 0 "ForOneFrame" false))
      (if (== (Utilities|GetClass (.HitActor (Collision|BreakHitResult _outhit))) "/Game/BP_fyk/BP_Building.BP_Building_C")
        (bind _asbp_building (Utilities|Casting|CastToBP_Building (.HitActor (Collision|BreakHitResult _outhit))))
        (Utilities|Array|RemoveItem _buildings _asbp_building)
        (Development|PrintString (Utilities|String|ToString(Integer) (Utilities|Array|Length _buildings)))
        (CallFunction|SetGridSituationFree (Variables|/Game/BP_fyk/BP_Building.BP_Building_C|GetXLength _asbp_building) (Variables|/Game/BP_fyk/BP_Building.BP_Building_C|GetYLength _asbp_building) (Variables|/Game/BP_fyk/BP_Building.BP_Building_C|GetXposition _asbp_building) (Variables|/Game/BP_fyk/BP_Building.BP_Building_C|GetYposition _asbp_building))
        (Actor|DestroyActor _asbp_building)))
    (:NewEnumerator3
      ;[1 1 1] 放置鱼类
      (bind _outhit_2 (Collision|LineTraceByChannel _worldlocation (+ _worldlocation (* _worlddirection 10000)) "TraceTypeQuery1" false 0 "ForOneFrame" false))
      (if (== (Utilities|GetClass (.HitActor (Collision|BreakHitResult _outhit_2))) "/Game/BP_fyk/BP_Building.BP_Building_C")
        (bind _asbp_building_2 (Utilities|Casting|CastToBP_Building (.HitActor (Collision|BreakHitResult _outhit_2))))
        (Default|AddFish _asbp_building_2 (.fishname _curfishinfo) (.viewvalue _curfishinfo))
        (else
          (Development|PrintString "can't put here"))))))

(event Custom|printOcupidGridNum
  (for _array_element (Variables|Default|GetGridSituation)
    (if (Math|Boolean|Equal(Boolean) _array_element true)
      (Variables|Default|SetCounter (+ (Variables|Default|GetCounter) 1))))
  (Development|PrintString (Utilities|String|ToString(Integer) (Variables|Default|GetCounter)))
  (Variables|Default|SetCounter 0))

(event EventBeginPlay
  (bind _plane (Variables|Default|GetPlane))
  (bind _relativelocation (Variables|/Script/Engine.SceneComponent|GetRelativeLocation _plane))
  ;[1 1 1] 初始化
  (Variables|Default|SetMyBuildMode "NewEnumerator0")
  (bind _asbp_game_instance (Utilities|Casting|CastToBP_GameInstance (Game|GetGameInstance)))
  (Variables|Default|SetMyGameInstance _asbp_game_instance)
  (Variables|Default|SetCellSizeX (/ (* 2 (.x _relativelocation)) (Variables|Default|GetXCount)))
  (Variables|Default|SetCellSizeY (/ (* 2 (.y _relativelocation)) (Variables|Default|GetYCount)))
  (CallFunction|ChangeCurBuildingbyName "Type1_1")
  (CallFunction|ChangeCurHoldFishbyName "Type1")
  (CallFunction|ClearGrid))

(event EventTick
  (params (DeltaSeconds :type Float%20%28single-precision%29))
  (bind _returnvalue (Game|GetPlayerController 0))
  (bind _returnvalue_2 (|CaculateLocation))
  (bind _previewfish (Variables|Default|GetPreviewFish))
  (bind (_worldlocation _worlddirection) (Game|Player|ConvertMouseLocationToWorldSpace _returnvalue))
  ;[1 1 1] 获取当前指向格子位置并设置preview位置
  (switch Utilities|FlowControl|Switch|SwitchonGameMode (Variables|/Game/BP_fyk/BP_boat.BP_boat_C|GetGameMode (Variables|/Game/BP_xyl/Inventory/GameFramework/BP_GameInstance.BP_GameInstance_C|GetPlayerBoat (Variables|Default|GetMyGameInstance)))
    (:NewEnumerator3
      (bind _outhit (Collision|LineTraceByChannel _worldlocation (+ _worldlocation (* _worlddirection 10000)) "TraceTypeQuery1" false (Variables|Default|GetBuildings) "ForOneFrame" false))
      (if (== (.HitActor (Collision|BreakHitResult _outhit)) self)
        (Variables|Default|SetCurMouseCell (Math|Vector2D|MakeVector2D (Math|Conversions|ToFloat(Integer) (Math|Float|Truncate (/ (.x (- (.Location (Collision|BreakHitResult _outhit)) (Transformation|GetActorLocation))) (Variables|Default|GetCellSizeX)))) (Math|Conversions|ToFloat(Integer) (Math|Float|Truncate (/ (.y (- (.Location (Collision|BreakHitResult _outhit)) (Transformation|GetActorLocation))) (Variables|Default|GetCellSizeY))))))
        (Utilities|FlowControl|Sequence
          (:then_0
            (if (Math|Vector|Equal(Vector) (Variables|Default|GetCurLocation) _returnvalue_2 0.0001)
              (switch Utilities|FlowControl|Switch|SwitchonBuildMode (Variables|Default|GetMyBuildMode)
                (:NewEnumerator1
                  (bind _movingline (Timeline|PreviewMoving Play)
                    (:Update
                      (Transformation|SetActorLocation (Variables|Default|GetpreviewBuilding_ver2) (Math|Vector|Lerp(Vector) (Transformation|GetActorLocation (Variables|Default|GetpreviewBuilding_ver2)) (Variables|Default|GetCurLocation) _movingline) false false))))
                (:NewEnumerator3
                  (bind _movingline_2 (Timeline|FishPreviewMoving Play)
                    (:Update
                      (Transformation|SetActorLocation _previewfish (Math|Vector|Lerp(Vector) (Transformation|GetActorLocation _previewfish) (Variables|Default|GetCurLocation) _movingline_2) false false)))))
              (else
                (Variables|Default|SetCurLocation _returnvalue_2)
                (Utilities|FlowControl|Sequence
                  (:then_0
                    (Timeline|PreviewMoving SetNewTime))
                  (:then_1
                    (Timeline|FishPreviewMoving SetNewTime)))))))))))

(event Input|KeyboardEvents|B
  (params (Key :type Key%20Structure :default "None"))
  (bind _mybuildmode (Variables|Default|GetMyBuildMode))
  ;[1 1 1] 进入建造模式
  (:Pressed
    (switch Utilities|FlowControl|Switch|SwitchonGameMode (Variables|/Game/BP_fyk/BP_boat.BP_boat_C|GetGameMode (Variables|/Game/BP_xyl/Inventory/GameFramework/BP_GameInstance.BP_GameInstance_C|GetPlayerBoat (Variables|Default|GetMyGameInstance)))
      (:NewEnumerator3
        (if (Utilities|Enum|Equal(Enum) _mybuildmode "NewEnumerator1")
          (CallFunction|ExitCurBuildMode _mybuildmode)
          (CallFunction|ChangeMode "NewEnumerator0")
          (Development|PrintString "Idle")
          (else
            (CallFunction|ExitCurBuildMode _mybuildmode)
            (CallFunction|ChangeMode "NewEnumerator1")
            (Development|PrintString "Build")))))))

(event Input|KeyboardEvents|4
  (params (Key :type Key%20Structure :default "None"))
  ;[1 1 1] 改变建筑类型
  (:Pressed
    (switch Utilities|FlowControl|Switch|SwitchonBuildMode (Variables|Default|GetMyBuildMode)
      (:NewEnumerator1
        (CallFunction|ChangeCurBuildingbyName "Type1_1"))
      (:NewEnumerator3
        (CallFunction|ChangeCurHoldFishbyName "最普通的鱼")))))

(event Input|KeyboardEvents|5
  (params (Key :type Key%20Structure :default "None"))
  ;[1 1 1] 改变建筑类型
  (:Pressed
    (switch Utilities|FlowControl|Switch|SwitchonBuildMode (Variables|Default|GetMyBuildMode)
      (:NewEnumerator1
        (CallFunction|ChangeCurBuildingbyName "Type1_2"))
      (:NewEnumerator3
        (CallFunction|ChangeCurHoldFishbyName "常见的食用鱼")))))

(event Input|KeyboardEvents|6
  (params (Key :type Key%20Structure :default "None"))
  ;[1 1 1] 改变建筑类型
  (:Pressed
    (switch Utilities|FlowControl|Switch|SwitchonBuildMode (Variables|Default|GetMyBuildMode)
      (:NewEnumerator1
        (CallFunction|ChangeCurBuildingbyName "Type2_2"))
      (:NewEnumerator3
        (CallFunction|ChangeCurHoldFishbyName "有观赏价值的鱼")))))

(event Input|KeyboardEvents|X
  (params (Key :type Key%20Structure :default "None"))
  (bind _mybuildmode (Variables|Default|GetMyBuildMode))
  ;[1 1 1] 进入删除模式
  (:Pressed
    (switch Utilities|FlowControl|Switch|SwitchonGameMode (Variables|/Game/BP_fyk/BP_boat.BP_boat_C|GetGameMode (Variables|/Game/BP_xyl/Inventory/GameFramework/BP_GameInstance.BP_GameInstance_C|GetPlayerBoat (Variables|Default|GetMyGameInstance)))
      (:NewEnumerator3
        (if (Utilities|Enum|Equal(Enum) _mybuildmode "NewEnumerator2")
          (CallFunction|ExitCurBuildMode _mybuildmode)
          (CallFunction|ChangeMode "NewEnumerator0")
          (Development|PrintString "Idle")
          (else
            (CallFunction|ExitCurBuildMode _mybuildmode)
            (CallFunction|ChangeMode "NewEnumerator2")
            (Development|PrintString "Delete")))))))

(fn ConstructionScript
  (bind _xcount (Variables|Default|GetXCount))
  (bind _ycount (Variables|Default|GetYCount))
  (bind _plane (Variables|Default|GetPlane))
  (bind _relativelocation (Variables|/Script/Engine.SceneComponent|GetRelativeLocation _plane))
  (bind _relativescale3d (Variables|/Script/Engine.SceneComponent|GetRelativeScale3D _plane))
  (Utilities|FlowControl|Sequence
    (:then_0
      (for _index (range 0 (Math|Float|Truncate _xcount))
        (bind _returnvalue (AddComponent|AddStaticMeshComponent false (Math|Transform|MakeTransform (Math|Vector|MakeVector (* _index (/ (* 2 (.x _relativelocation)) _xcount)) (.y _relativelocation) (+ (.z _relativelocation) 1.0)) "0, 0, 0" (Math|Vector|MakeVector 0.04 (.y _relativescale3d) 1.0))))
        (Utilities|Array|SetArrayElem (Variables|Default|GetLines) _index _returnvalue)))
    (:then_1
      (for _index_2 (range 0 (Math|Float|Truncate _ycount))
        (AddComponent|AddStaticMeshComponent false (Math|Transform|MakeTransform (Math|Vector|MakeVector (.x _relativelocation) (* _index_2 (/ (* 2 (.y _relativelocation)) _ycount)) (+ (.z _relativelocation) 1.0)) "0, 0, 0" (Math|Vector|MakeVector (.x _relativescale3d) 0.04 1.0)))))
    (:then_2
      (Variables|Default|SetcurBuildingType "NewEnumerator0")
      (Variables|Default|SetCurBuildingXLength 1.0)
      (Variables|Default|SetCurBuildingYLength 1.0)
      (for _index_3 (range 0 (Math|Float|Truncate (Variables|Default|GetXCount)))
        (for _index_4 (range 0 (Math|Float|Truncate (Variables|Default|GetYCount)))
          (Utilities|Array|Add (Variables|Default|GetGridSituation) false))))))

(fn SetGridSituation
  (params (NewParam :type Vector%202D%20Structure))
  (bind _curmousecell (Variables|Default|GetCurMouseCell))
  (for _index (range (Math|Float|Truncate (.x _curmousecell)) (Math|Float|Truncate (+ (.x _curmousecell) (- (.x NewParam) 1.0))))
    (for _index_2 (range (Math|Float|Truncate (.y _curmousecell)) (Math|Float|Truncate (+ (.y _curmousecell) (- (.y NewParam) 1.0))))
      (Utilities|Array|SetArrayElem (Variables|Default|GetGridSituation) (+ _index (Math|Float|Truncate (* _index_2 (Variables|Default|GetXCount)))) true))))

(fn ChangeCurBuildingbyName
  (params (BuildingName :type String))
  (bind _outrownames (DataTable|GetDataTableRowNames "/Game/BP_fyk/Data/DT_BuildingTypes.DT_BuildingTypes"))
  (bind _array_element (Utilities|Array|ForEachLoopwithBreak _outrownames)
    (:LoopBody
      (bind _returnvalue (Utilities|GetDataTableRow "/Game/BP_fyk/Data/DT_BuildingTypes.DT_BuildingTypes" _array_element)
        (:then
          (if (Utilities|Enum|Equal(Enum) BuildingName (.Name (Utilities|Struct|BreakStruct_building _returnvalue)))
            (Variables|Default|SetCurBuildingInfo _returnvalue)
            (Default|ChangeMesh (Variables|Default|GetpreviewBuilding_ver2) (.Mesh (Utilities|Struct|BreakStruct_building _returnvalue)) (.XLength (Utilities|Struct|BreakStruct_building _returnvalue)) (.YLength (Utilities|Struct|BreakStruct_building _returnvalue)))
            (Variables|Default|SetCurBuildingXLength (.XLength (Utilities|Struct|BreakStruct_building _returnvalue)))
            (Variables|Default|SetCurBuildingYLength (.YLength (Utilities|Struct|BreakStruct_building _returnvalue)))))))))

(fn CheckGrid
  (bind _curmousecell (Variables|Default|GetCurMouseCell))
  (for _index (range (Math|Float|Truncate (.x _curmousecell)) (Math|Float|Truncate (+ (.x _curmousecell) (- (Variables|Default|GetCurBuildingXLength) 1.0))))
    (for _index_2 (range (Math|Float|Truncate (.y _curmousecell)) (Math|Float|Truncate (+ (.y _curmousecell) (- (Variables|Default|GetCurBuildingYLength) 1.0))))
      (if (Math|Boolean|Equal(Boolean) (Utilities|Array|Get(acopy) (Variables|Default|GetGridSituation) (+ _index (Math|Float|Truncate (* _index_2 (Variables|Default|GetXCount))))) true)
        (return false))))
  (return true))

(fn ClearGrid
  (bind _gridsituation (Variables|Default|GetGridSituation))
  (for (_ _array_index) _gridsituation
    (Utilities|Array|SetArrayElem _gridsituation _array_index false)))

(fn SetGridSituationFree
  (params (XLength :type Float%20%28single-precision%29) (YLength :type Float%20%28single-precision%29) (Xposition :type Float%20%28single-precision%29) (Yposition :type Float%20%28single-precision%29))
  (for _index (range (Math|Float|Truncate Xposition) (Math|Float|Truncate (+ Xposition (- XLength 1.0))))
    (for _index_2 (range (Math|Float|Truncate Yposition) (Math|Float|Truncate (+ Yposition (- YLength 1.0))))
      (Utilities|Array|SetArrayElem (Variables|Default|GetGridSituation) (+ _index (Math|Float|Truncate (* _index_2 (Variables|Default|GetXCount)))) false))))

(fn ExitCurBuildMode
  (params (Mode :type BuildMode%20Enum :default "NewEnumerator0"))
  (switch Utilities|FlowControl|Switch|SwitchonBuildMode Mode
    (:NewEnumerator1
      (Rendering|SetVisibility (Variables|/Game/BP_fyk/BP_PreviewBuilding.BP_PreviewBuilding_C|GetBuilding (Variables|Default|GetpreviewBuilding_ver2)) false false))
    (:NewEnumerator3
      (Rendering|SetVisibility (Variables|/Game/BP_fyk/BP_previewFish.BP_previewFish_C|GetFish (Variables|Default|GetPreviewFish)) false false))))

(fn ChangeMode
  (params (NewMode :type BuildMode%20Enum :default "NewEnumerator0"))
  (switch Utilities|FlowControl|Switch|SwitchonBuildMode NewMode
    (:NewEnumerator0
      (Variables|Default|SetMyBuildMode "NewEnumerator0"))
    (:NewEnumerator1
      (Variables|Default|SetMyBuildMode "NewEnumerator1")
      (Rendering|SetVisibility (Variables|/Game/BP_fyk/BP_PreviewBuilding.BP_PreviewBuilding_C|GetBuilding (Variables|Default|GetpreviewBuilding_ver2)) true false))
    (:NewEnumerator2
      (Variables|Default|SetMyBuildMode "NewEnumerator2"))
    (:NewEnumerator3
      (Variables|Default|SetMyBuildMode "NewEnumerator3")
      (Rendering|SetVisibility (Variables|/Game/BP_fyk/BP_previewFish.BP_previewFish_C|GetFish (Variables|Default|GetPreviewFish)) true false)
      (Variables|Default|SetCurBuildingXLength 1.0)
      (Variables|Default|SetCurBuildingYLength 1.0))))

(fn ChangeCurHoldFishbyName
  (params (FishName :type String))
  (bind _outrownames (DataTable|GetDataTableRowNames "/Game/BP_fyk/Data/DT_FishTypes.DT_FishTypes"))
  (bind _array_element (Utilities|Array|ForEachLoopwithBreak _outrownames)
    (:LoopBody
      (bind _returnvalue (Utilities|GetDataTableRow "/Game/BP_fyk/Data/DT_FishTypes.DT_FishTypes" _array_element)
        (:then
          (if (Utilities|Enum|Equal(Enum) FishName (.FishName (Utilities|Struct|Breakstruct_fishType _returnvalue)))
            (Variables|Default|SetCurFishInfo _returnvalue)
            (Components|StaticMesh|SetStaticMesh (Variables|/Game/BP_fyk/BP_previewFish.BP_previewFish_C|GetFish (Variables|Default|GetPreviewFish)) (.FishMesh (Utilities|Struct|Breakstruct_fishType _returnvalue)))))))))

(fn CaculateAllIncome
  (for _array_element (Variables|Default|GetBuildings)
    (if (> (Variables|/Game/BP_fyk/BP_Building.BP_Building_C|GetCurFishNum _array_element) 0.0)
      (bind _value (Default|CalculateValuePerDay _array_element))
      (LocalVariables|SetIncomeCounter (+ _value (LocalVariables|GetIncomeCounter)))
      (LocalVariables|SetIncomeCounter (- (LocalVariables|GetIncomeCounter) (Variables|/Game/BP_fyk/BP_Building.BP_Building_C|GetMaintainCost _array_element)))))
  (return (- (LocalVariables|GetIncomeCounter) (Variables|Default|GetDailyCost))))
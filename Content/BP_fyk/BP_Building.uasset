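; BP_Building is a building that holds fish up to a capacity and earns daily value from their view values.
; On BeginPlay, a timeline animates the actor's scale around its normal size.
; AddFish appends a name and value struct to the fish array, or prints that the cabin is filled.
; CalculateValuePerDay sums the stored view values, applies a multiplier, and prints and returns the result.
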(event EventBeginPlay
  (bind _newtrack_0 (Timeline|Timeline_0 PlayFromStart)
    (:Update
      (Transformation|SetActorScale3D (Math|Vector|Lerp(Vector) "0.800000,0.800000,0.800000" "1.200000,1.200000,1.200000" _newtrack_0)))))

(event Collision|EventActorBeginOverlap
  (params (OtherActor :type Actor%20Object%20Reference)))

(event EventTick
  (params (DeltaSeconds :type Float%20%28single-precision%29)))

(fn ConstructionScript)

(fn AddFish
  (params (FishName :type String) (FishValue :type Float%20%28single-precision%29))
  (bind _fisharray (Variables|Default|GetFishArray))
  (if (< (Variables|Default|GetCurFishNum) (Variables|Default|GetFishCapacity))
    (Variables|Default|SetCurFishNum (+ (Variables|Default|GetCurFishNum) 1.0))
    (Utilities|Array|Add _fisharray (Utilities|Struct|Makestruct_fish_display FishName FishValue))
    (Development|PrintString (Utilities|String|ToString(Integer) (Utilities|Array|Length _fisharray)))
    (else
      (Development|PrintString "this cabin is filled"))))

(fn CalculateValuePerDay
  (for _array_element (Variables|Default|GetFishArray)
    (LocalVariables|SetFishValueCount (+ (LocalVariables|GetFishValueCount) (.ViewValue (Utilities|Struct|Breakstruct_fish_display _array_element)))))
  (Development|PrintString (Utilities|String|ToString(Float) (* (LocalVariables|GetFishValueCount) (Variables|Default|GetViewValueTimes))))
  (return (* (LocalVariables|GetFishValueCount) (Variables|Default|GetViewValueTimes))))
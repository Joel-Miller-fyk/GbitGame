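; Player controller for the inventory system that creates the main UI widget at BeginPlay and drives it from hard-wired keys.
; Tab toggles the inventory along with input mode and cursor, while R and T hide and show the hotbar and equipment sockets.
; Q and E open buy and sell shop widgets in UI-only mode, and K prints one item type's GameInstance data for debugging.
; Helper functions return item widgets from inventory and equipment slots.
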(event EventBeginPlay
  (bind _returnvalue (UserInterface|CreateWidget "/Game/BP_xyl/Inventory/UI/W_Main.W_Main_C"))
  (bind _output_get (Variables|Default|SetUI _returnvalue))
  (UserInterface|Viewport|AddtoViewport _output_get 0))

(event Input|KeyboardEvents|T
  (params (Key :type Key%20Structure))
  (bind _ui (Variables|Default|GetUI))
  ;[1 1 1] 显示/不显示控件
  (:Pressed
    (Widget|SetVisibility (Variables|/Game/BP_xyl/Inventory/UI/W_Main.W_Main_C|GetW_Hotbar _ui) "Visible")
    (Widget|SetVisibility (Variables|/Game/BP_xyl/Inventory/UI/W_Main.W_Main_C|GetW_EquipmentSocket _ui) "Visible")))

(event Input|KeyboardEvents|K
  (params (Key :type Key%20Structure))
  (:Pressed
    (bind _props (Class|InterfaceGameInstance|GetInventorybyPropType(Message) (Game|GetGameInstance) "NewEnumerator0"))
    (for _array_element _props
      (Development|PrintString (Utilities|String|Append "背包位置" (Utilities|String|ToString(Integer) (.InventoryIndex (Utilities|Struct|BreakS_InventoryItem _array_element))) "--ID" (Utilities|String|ToString(Integer) (.ID (Utilities|Struct|BreakS_InventoryItem _array_element))) "--数量" (Utilities|String|ToString(Integer) (.Quantity (Utilities|Struct|BreakS_InventoryItem _array_element)))) true true "(R=0.000000,G=0.660000,B=1.000000,A=1.000000)" 5.0))))

(event Input|KeyboardEvents|Tab
  (params (Key :type Key%20Structure))
  (bind _self self)
  (bind _ui (Variables|Default|GetUI))
  (bind _w_inventory (Variables|/Game/BP_xyl/Inventory/UI/W_Main.W_Main_C|GetW_Inventory _ui))
  (:Pressed
    (if (Widget|IsVisible _w_inventory)
      (Widget|SetVisibility _w_inventory "Collapsed")
      (Input|SetInputModeGameOnly _self)
      (Variables|Default|SetbShowMouseCursor false)
      (else
        (Widget|SetVisibility _w_inventory "Visible")
        (Input|SetInputModeGameandUI _self _w_inventory "DoNotLock" true)
        (Variables|Default|SetbShowMouseCursor true)))))

(event Input|KeyboardEvents|Q
  (params (Key :type Key%20Structure))
  (bind _returnvalue (Game|GetPlayerController 0))
  ;[1 1 1] 商店测试
  (:Pressed
    (bind _returnvalue_2 (UserInterface|CreateWidget "/Game/BP_xyl/Inventory/UI/W_Shop.W_Shop_C"))
    (UserInterface|Viewport|AddtoViewport _returnvalue_2 0)
    (Input|SetInputModeUIOnly _returnvalue _returnvalue_2 "DoNotLock")
    (Variables|/Script/Engine.PlayerController|SetbShowMouseCursor _returnvalue true)))

(event Input|KeyboardEvents|E
  (params (Key :type Key%20Structure))
  (bind _returnvalue (Game|GetPlayerController 0))
  ;[1 1 1] 卖出物品
  (:Pressed
    (bind _returnvalue_2 (UserInterface|CreateWidget "/Game/BP_xyl/Inventory/UI/W_SellShop.W_SellShop_C"))
    (UserInterface|Viewport|AddtoViewport _returnvalue_2 0)
    (Input|SetInputModeUIOnly _returnvalue _returnvalue_2 "DoNotLock")
    (Variables|/Script/Engine.PlayerController|SetbShowMouseCursor _returnvalue true)))

(event Input|KeyboardEvents|R
  (params (Key :type Key%20Structure))
  (bind _ui (Variables|Default|GetUI))
  ;[1 1 1] 显示/不显示控件
  (:Pressed
    (Widget|SetVisibility (Variables|/Game/BP_xyl/Inventory/UI/W_Main.W_Main_C|GetW_Hotbar _ui) "Collapsed")
    (Widget|SetVisibility (Variables|/Game/BP_xyl/Inventory/UI/W_Main.W_Main_C|GetW_EquipmentSocket _ui) "Collapsed")))

(fn ConstructionScript)

(fn GetEquipmentSocketItem
  (params (Index :type Integer))
  (bind _ui (Variables|Default|GetUI))
  (Utilities|IsValid _ui
    (:Is%20Valid
      (bind _asw_inventory_item (Utilities|Casting|CastToW_InventoryItem (Class|PanelWidget|GetChildat (Variables|/Game/BP_xyl/Inventory/UI/W_EquipmentSocket.W_EquipmentSocket_C|GetUniformGrid_AllEquipment (Variables|/Game/BP_xyl/Inventory/UI/W_Main.W_Main_C|GetW_EquipmentSocket _ui)) Index)))
      (return _asw_inventory_item))))

(fn GetInventoryItem
  (params (Type :type E_PropType%20Enum :default "NewEnumerator0") (Index :type Integer))
  (bind _ui (Variables|Default|GetUI))
  (Utilities|IsValid _ui
    (:Is%20Valid
      (bind _asw_inventory_item (Default|GetInventoryItem (Variables|/Game/BP_xyl/Inventory/UI/W_Main.W_Main_C|GetW_Inventory _ui) Type Index))
      (return _asw_inventory_item))))
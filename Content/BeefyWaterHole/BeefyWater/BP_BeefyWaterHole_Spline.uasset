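; Spline-based water actor for BeefyWaterHole that builds a river surface along the editable RiverSpline.
; The construction script assigns RiverSpline as the inherited WaterComponent, then creates one spline mesh per segment with the configured mesh, material and scale.
; Each segment follows the spline's local points and tangents, with query-only collision set to block WorldStatic.
; BeginPlay and overlap events only forward to the parent class.
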(event EventBeginPlay
  (|CallParentFunction))

(event Collision|EventActorBeginOverlap
  (params (OtherActor :type Actor%20Object%20Reference))
  (|CallParentFunction OtherActor))

(event Collision|EventActorEndOverlap
  (params (OtherActor :type Actor%20Object%20Reference))
  (|CallParentFunction OtherActor))

(fn ConstructionScript
  (|CallParentFunction)
  (Variables|Default|SetWaterComponent (Variables|Default|GetRiverSpline))
  (for _index (range 0 (- (Spline|GetNumberOfSplinePoints (Variables|Default|GetRiverSpline)) 2))
    (CallFunction|CreateSplineMesh _index)))

(fn CreateSplineMesh
  (params (MeshIndex :type Integer))
  (bind _returnvalue (+ MeshIndex 1))
  (bind _mesh_scale (Variables|Default|GetMesh%20Scale))
  (bind _riverspline (Variables|Default|GetRiverSpline))
  (bind (_location _tangent) (Spline|GetLocationandTangentatSplinePoint _riverspline _returnvalue "Local"))
  (bind (_location_2 _tangent_2) (Spline|GetLocationandTangentatSplinePoint _riverspline MeshIndex "Local"))
  (bind _returnvalue_2 (AddComponent|AddSplineMeshComponent false))
  (SplineMesh|SetStartScale _returnvalue_2 (Math|Vector2D|MakeVector2D _mesh_scale _mesh_scale) true :!class /Script/Engine.SplineMeshComponent)
  (SplineMesh|SetEndScale _returnvalue_2 (Math|Vector2D|MakeVector2D _mesh_scale _mesh_scale) true :!class /Script/Engine.SplineMeshComponent)
  (Transformation|AttachComponentToComponent _returnvalue_2 (Variables|Default|GetDefaultSceneRoot) "None" "KeepRelative" "KeepRelative" "KeepRelative" true)
  (Components|StaticMesh|SetStaticMesh _returnvalue_2 (Variables|Default|GetWater%20Mesh))
  (Rendering|Material|SetMaterial _returnvalue_2 0 (Variables|Default|GetWater%20Material))
  (Collision|SetCollisionEnabled _returnvalue_2 "QueryOnly")
  (Collision|SetCollisionResponsetoChannel _returnvalue_2 "ECC_WorldStatic" "ECR_Block")
  (SplineMesh|SetStartandEnd _returnvalue_2 _location_2 _tangent_2 _location _tangent true :!class /Script/Engine.SplineMeshComponent))